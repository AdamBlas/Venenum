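; Player blob character with camera-relative movement, scroll zoom and size-based split, merge and possess skills.
; Q tap spawns a BP_Blob by shrinking and hold calls an empty shoot stub; E tap merges with an overlapped blob and hold possesses one by swapping location and size.
; Tick scans all blobs for possession targets using a view angle that widens with proximity, and updates HUD availability and radial hold-progress materials.
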(event `self.Trigger.OnComponentBeginOverlap`
  (params (OverlappedComponent :type "PrimitiveComponent Object Reference") (OtherActor :type "Actor Object Reference") (OtherComp :type "PrimitiveComponent Object Reference") (OtherBodyIndex :type Integer) (bFromSweep :type Boolean) (SweepResult :type "HitResult Structure (by ref)"))
  ;[1 1 1] On Overlap
  (`self.Check If Overlapped Blob` OtherActor true))

(event `self.Trigger.OnComponentEndOverlap`
  (params (OverlappedComponent :type "PrimitiveComponent Object Reference") (OtherActor :type "Actor Object Reference") (OtherComp :type "PrimitiveComponent Object Reference") (OtherBodyIndex :type Integer))
  ;[1 1 1] On Overlap
  (`self.Check If Overlapped Blob` OtherActor))

(event `InputAxis|MouseWheel`
  (params (AxisValue :type "Float (single-precision)"))
  ;[1 1 1] SpringArm Extension
  (bind _result (`/Engine/EditorBlueprintResources/StandardMacros.NegateFloat` AxisValue)
    (:`  `
      (set `SpringArmComponent.TargetArmLength` (`KismetMathLibrary.FClamp` (+ (* (`self.Mouse Scroll Sensitivity`) _result) (`SpringArmComponent.TargetArmLength` (`self.SpringArm`))) (`self.Min SpringArm`) (`self.Max SpringArm`)) (`self.SpringArm`)))))

(event `InputAction|Interaction1`
  (params (Key :type "Key Structure"))
  (:`Pressed`
    (set `self.E Hold` true))
  (:`Released`
    (set `self.E Hold` false)
    (`self.Manage E Blob Skills`)))

(event `InputAxis|CameraRight`
  (params (AxisValue :type "Float (single-precision)"))
  ;[1 1 1] Camera Rotation
  (`self.AddControllerYawInput` (* AxisValue (`self.Camera Sensitivity`))))

(event `InputAction|Interaction2`
  (params (Key :type "Key Structure"))
  (:`Pressed`
    (set `self.Q Hold` true))
  (:`Released`
    (set `self.Q Hold` false)
    (`self.Manage Q Blob Skills`)))

(event `InputAxis|CameraUp`
  (params (AxisValue :type "Float (single-precision)"))
  ;[1 1 1] Camera Rotation
  (`self.AddControllerPitchInput` (* (`self.Camera Sensitivity`) AxisValue)))

(event `InputAxis|MoveForward`
  (params (AxisValue :type "Float (single-precision)"))
  ;[1 1 1] Movement
  (`self.AddMovementInput` (`KismetMathLibrary.GetForwardVector` (`KismetMathLibrary.MakeRotator` 0.0 0.0 (.yaw (`self.GetControlRotation`)))) AxisValue))

(event `InputAxis|MoveRight`
  (params (AxisValue :type "Float (single-precision)"))
  ;[1 1 1] Movement
  (`self.AddMovementInput` (`KismetMathLibrary.GetRightVector` (`KismetMathLibrary.MakeRotator` 0.0 0.0 (.yaw (`self.GetControlRotation`)))) AxisValue))

(event `self.ReceiveTick`
  (params (DeltaSeconds :type "Float (single-precision)"))
  ;[1 1 1] Tick
  (`self.Manage Q Hold` DeltaSeconds)
  (`self.Manage E Hold` DeltaSeconds)
  (`self.Check For Blobs To Possess`)
  (`self.Update HUD Colors`))

(event `self.ReceiveBeginPlay`
  ;[1 1 1] Begin Play
  (`self.Init HUD`)
  (`self.Set Spawn Rate` 15.0))

(event `Init HUD`
  (`KismetSystemLibrary.Delay` 0.0)
  (`self.Create DMI`)
  (`self.Update HUD Size Value`))

(fn `Angle Between Vectors`
  (params (`Vector A` :type "Vector Structure") (`Vector B` :type "Vector Structure"))
  (returns (`Angle In Degrees` :type "Float (double-precision)") (`Angle In Radians` :type "Float (double-precision)"))
  (bind _returnvalue (`KismetMathLibrary.Acos` (`KismetMathLibrary.Dot_VectorVector` (`KismetMathLibrary.Normal` `Vector A` 0.0) (`KismetMathLibrary.Normal` `Vector B` 0.0))))
  (return (* _returnvalue 57.29578) _returnvalue))

(fn `Check For Blobs To Possess`
  (locals (`Min Distance` :type "Float (double-precision)"))
  (set `local.Min Distance` 1200.0)
  (bind _outactors (`GameplayStatics.GetAllActorsOfClass` "/Game/Assets/Blueprints/BP_Blob.BP_Blob_C"))
  (for _array_element _outactors
    (if (not (`self.ActorHasTag` _array_element "Player"))
      (bind _returnvalue (`KismetMathLibrary.MakeVector` (.x (- (`self.K2_GetActorLocation` _array_element) (`self.K2_GetActorLocation`))) (.y (- (`self.K2_GetActorLocation` _array_element) (`self.K2_GetActorLocation`)))))
      (bind _returnvalue_2 (`KismetMathLibrary.VSize` _returnvalue))
      (if (<= _returnvalue_2 (`local.Min Distance`))
        (bind _angle_in_degrees (`self.Angle Between Vectors` _returnvalue (`KismetMathLibrary.MakeVector` (.x (`KismetMathLibrary.GetForwardVector` (`KismetMathLibrary.MakeRotator` 0.0 0.0 (.yaw (`self.GetControlRotation`))))) (.y (`KismetMathLibrary.GetForwardVector` (`KismetMathLibrary.MakeRotator` 0.0 0.0 (.yaw (`self.GetControlRotation`))))))))
        (bind _output_get (set `self.Can Possess Blob` (<= _angle_in_degrees (* (/ (`local.Min Distance`) _returnvalue_2) 10.0))))
        (if _output_get
          (set `self.Blob To Possess` _array_element)
          (break)
          (else
            (set `self.Blob To Possess` null)))
        (else
          (set `self.Can Possess Blob` false))))))

(fn `Check If Overlapped Blob`
  (params (Other :type "Actor Object Reference") (`Start Overlap` :type Boolean))
  (if (`self.ActorHasTag` Other "Blob")
    (set `self.Is Inside Blob` `Start Overlap`)
    (bind _asbp_blob (cast `/Game/Assets/Blueprints/BP_Blob` Other))
    (set `self.Blob To Merge` _asbp_blob)))

(fn `Create DMI`
  (bind _returnvalue (`KismetMaterialLibrary.CreateDynamicMaterialInstance` "/Game/Assets/GFX/Materials/M_CircleProgressBar.M_CircleProgressBar" "None" "Transient"))
  (bind _output_get (set `/Game/Assets/Blueprints/Widgets_BPs/W_HUD.Q Hold DMI` _returnvalue (`self.HUD Widget`)))
  (set `self.Q Hold DMI` _output_get)
  (bind _returnvalue_2 (`KismetMaterialLibrary.CreateDynamicMaterialInstance` "/Game/Assets/GFX/Materials/M_CircleProgressBar.M_CircleProgressBar" "None" "Transient"))
  (bind _output_get_2 (set `/Game/Assets/Blueprints/Widgets_BPs/W_HUD.E Hold DMI` _returnvalue_2 (`self.HUD Widget`)))
  (set `self.E Hold DMI` _output_get_2))

(fn `Manage E Blob Skills`
  (if (> (`self.E Hold Value`) 1.0)
    (if (`self.Can Possess Blob`)
      (`self.Try To Possess Blob` (`self.Blob To Possess`))
      (`KismetSystemLibrary.PrintString` "Possess Blob"))
    (elif (`self.Is Inside Blob`)
      (bind _merged_successfully (`self.Try To Merge With Blob` (`self.Blob To Merge`)))
      (if _merged_successfully
        (`KismetSystemLibrary.PrintString` "MERGED WITH BLOB")
        (else
          (`KismetSystemLibrary.PrintString` "FAILED TO PRINT WITH BLOB"))))))

(fn `Manage E Hold`
  (params (`Delta Time` :type "Float (double-precision)"))
  (if (`self.E Hold`)
    (set `self.E Hold Value` (+ `Delta Time` (`self.E Hold Value`)))
    (else
      (set `self.E Hold Value` 0.0)))
  (`self.Manage Hold HUD` (`self.E Hold DMI`) (`self.E Hold Value`)))

(fn `Manage Hold HUD`
  (params (`Hold DMI` :type "MaterialInstanceDynamic Object Reference (by ref)") (Value :type "Float (double-precision) (by ref)"))
  (if (!= `Hold DMI` null)
    (`MaterialInstanceDynamic.SetScalarParameterValue` `Hold DMI` "Value" (`KismetMathLibrary.FClamp` (* (- Value 0.5) 2.0)))
    (else
      (return))))

(fn `Manage Q Blob Skills`
  (if (> (`self.Q Hold Value`) 1.0)
    (`self.Try To Shoot Blob`)
    (`KismetSystemLibrary.PrintString` "Shot Blob")
    (else
      (bind _left_blob (`self.Try To Leave Blob`))
      (if _left_blob
        (`KismetSystemLibrary.PrintString` "LEFT BLOB")
        (else
          (`KismetSystemLibrary.PrintString` "FAILED TO LEAVE BLOB"))))))

(fn `Manage Q Hold`
  (params (`Delta Time` :type "Float (double-precision)"))
  (if (`self.Q Hold`)
    (set `self.Q Hold Value` (+ `Delta Time` (`self.Q Hold Value`)))
    (else
      (set `self.Q Hold Value` 0.0)))
  (`self.Manage Hold HUD` (`self.Q Hold DMI`) (`self.Q Hold Value`)))

(fn `OnBlobOverlapEnd`
  (params (Blob :type "/Game/Assets/Blueprints/BP_Blob Object Reference"))
  (set `self.Is Inside Blob` false))

(fn `OnBlobOverlapStart`
  (params (Blob :type "/Game/Assets/Blueprints/BP_Blob Object Reference"))
  (set `self.Blob To Merge` Blob)
  (set `self.Is Inside Blob` true))

(fn `Try To Leave Blob`
  (returns (`Left Blob` :type Boolean))
  (bind _successfull (`self.Decrease Size`))
  (if _successfull
    (bind _returnvalue (`|SpawnActorFromClass` "/Game/Assets/Blueprints/BP_Blob.BP_Blob_C" (`self.GetTransform`) "AdjustIfPossibleButAlwaysSpawn" "OverrideRootScale" null null))
    (bind _trigger (`/Game/Assets/Blueprints/BP_Blob.Trigger` _returnvalue))
    (`SphereComponent.SetSphereRadius` _trigger (* (`SphereComponent.SphereRadius` _trigger) 5.0) true)
    (`self.Update HUD Size Value`)
    (return true)
    (else
      (return false))))

(fn `Try To Merge With Blob`
  (params (Blob :type "/Game/Assets/Blueprints/BP_Blob Object Reference"))
  (returns (`Merged successfully` :type Boolean))
  (if (`self.Is Inside Blob`)
    (bind _result (`self.Change Size` (`KismetMathLibrary.Clamp` (+ (`self.Size`) (`/Game/Assets/Blueprints/BP_Blob.Size` Blob)) 1 3)))
    (if _result
      (`self.Destory Blob Event` Blob)
      (`self.Update HUD Size Value`)
      (return true)
      (else
        (return false)))
    (else
      (return false))))

(fn `Try To Possess Blob`
  (params (`Blob To Possess` :type "/Game/Assets/Blueprints/BP_Blob Object Reference"))
  (locals (`Tmp Size` :type Integer) (`Tmp Location` :type "Vector Structure"))
  ;[1 1 1] Assign location and size to temporary variables
  (set `local.Tmp Location` (`self.K2_GetActorLocation` `Blob To Possess`))
  (set `local.Tmp Size` (`/Game/Assets/Blueprints/BP_Blob.Size` `Blob To Possess`))
  ;[1 1 1] Set location ad size of player to blob
  (`self.K2_SetActorLocation` `Blob To Possess` (`self.K2_GetActorLocation`) false false)
  (`self.Change Size` `Blob To Possess` (`self.Size`))
  ;[1 1 1] Set blob's location and size to player
  (`self.K2_SetActorLocation` (`local.Tmp Location`))
  (`self.Change Size` (`local.Tmp Size`))
  (`self.Update HUD Size Value`))

(fn `Try To Shoot Blob`)

(fn `Update HUD Colors`
  (bind _size (`self.Size`))
  (bind _returnvalue (> _size 1))
  (if (!= (`self.HUD Widget`) null)
    (set `/Game/Assets/Blueprints/Widgets_BPs/W_HUD.Shot Avaliable` _returnvalue (`self.HUD Widget`))
    (set `/Game/Assets/Blueprints/Widgets_BPs/W_HUD.Possess Avaliable` (`self.Can Possess Blob`) (`self.HUD Widget`))
    (set `/Game/Assets/Blueprints/Widgets_BPs/W_HUD.Split Avaliable` _returnvalue (`self.HUD Widget`))
    (set `/Game/Assets/Blueprints/Widgets_BPs/W_HUD.Merge Avaliable` (and (`self.Is Inside Blob`) (< _size 3)) (`self.HUD Widget`))))

(fn `Update HUD Size Value`
  (if (!= (`self.HUD Widget`) null)
    (set `/Game/Assets/Blueprints/Widgets_BPs/W_HUD.Size Value` (`self.Size`) (`self.HUD Widget`))))

(fn `UserConstructionScript`)