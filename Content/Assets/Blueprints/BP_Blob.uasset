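; Blob actor that drives a Niagara particle effect, setting its spawn rate on BeginPlay.
; Helper functions write the spawn rate and particle scale parameters, with ChangeSize rejecting out-of-range sizes and returning success.
; DestoryBlobEvent loops over an index as the spawn rate with a debug print, then destroys the actor; the Delay inside the for loop does not pause iteration.
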(event `self.ReceiveBeginPlay`
  (`self.Set Spawn Rate` 15.0))

(event `Destory Blob Event`
  (for _index (range 16)
    (`KismetSystemLibrary.Delay` 1.0)
    (`self.Set Spawn Rate` (`KismetMathLibrary.Conv_IntToDouble` _index))
    (`KismetSystemLibrary.PrintString` "Hello"))
  (`self.K2_DestroyActor`))

(fn `Change Size`
  (params (newSize :type Integer))
  (returns (result :type Boolean))
  (bind _returnvalue (`KismetMathLibrary.Conv_IntToDouble` newSize))
  (if (and (>= newSize 1) (<= newSize 3))
    (`NiagaraComponent.SetVariableVec2` (`self.Niagara GFX`) "Particle Scale" (`KismetMathLibrary.MakeVector2D` _returnvalue _returnvalue))
    (return true)
    (else
      (return false))))

(fn `Set Spawn Rate`
  (params (`New Rate` :type "Float (double-precision)"))
  (`FXSystemComponent.SetFloatParameter` (`self.Niagara GFX`) (`KismetStringLibrary.Conv_StringToName` "Spawn Rate") `New Rate`))

(fn `UserConstructionScript`)