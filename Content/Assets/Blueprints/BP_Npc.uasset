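; NPC that gets poisoned on overlap with a Player-tagged actor and is destroyed when its poison level fills.
; Each tick raises the level while poisoned or drains it otherwise, and turns the PoisonLevelBar widget, which receives the NPC as owner, toward the camera.
; On overlapping another BP_Npc, it overwrites that NPC's poison flag with its own AND the Poisonable tag check, so contact can also clear poison.
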(event `self.CapsuleComponent.OnComponentBeginOverlap`
  (params (OverlappedComponent :type "PrimitiveComponent Object Reference") (OtherActor :type "Actor Object Reference") (OtherComp :type "PrimitiveComponent Object Reference") (OtherBodyIndex :type Integer) (bFromSweep :type Boolean) (SweepResult :type "HitResult Structure (by ref)"))
  ;[1 1 1] On Collision
  (`self.TryToPoisonNpc` OtherActor)
  (`self.TryToSpreadPoison` OtherActor))

(event `self.ReceiveBeginPlay`
  ;[1 1 1] Start
  (`self.InitPoisonBar`))

(event `self.ReceiveTick`
  (params (DeltaSeconds :type "Float (single-precision)"))
  ;[1 1 1] Event Tick
  (`self.ManagePoisonLevel` DeltaSeconds)
  (`self.BollboardPoisonBar`))

(fn `BollboardPoisonBar`
  (bind _poison_level_bar (`self.Poison Level Bar`))
  (`SceneComponent.K2_SetWorldRotation` _poison_level_bar (`KismetMathLibrary.FindLookAtRotation` (`SceneComponent.K2_GetComponentLocation` _poison_level_bar) (`PlayerCameraManager.GetCameraLocation` (`GameplayStatics.GetPlayerCameraManager` 0))) false false))

(fn `InitPoisonBar`
  (bind _aspoison_level_bar (cast `/Game/Assets/Blueprints/Widgets_BPs/PoisonLevelBar` (`WidgetComponent.GetUserWidgetObject` (`self.Poison Level Bar`))))
  (set `/Game/Assets/Blueprints/Widgets_BPs/PoisonLevelBar.Owner` self _aspoison_level_bar))

(fn `ManagePoisonLevel`
  (params (deltaTime :type "Float (double-precision)"))
  (bind _poisonpercentage (`self.poisonPercentage`))
  (bind _returnvalue (* (`self.poisonSpeed`) deltaTime))
  (if (`self.isPoisoned`)
    (bind _output_get (set `self.poisonPercentage` (+ _poisonpercentage _returnvalue))) ; Increase
    (if (>= _output_get 1.0)
      (`self.K2_DestroyActor`))
    (elif (> (`self.poisonPercentage`) 0.0)
      (set `self.poisonPercentage` (- _poisonpercentage _returnvalue)) ; Decrease
    )))

(fn `TryToPoisonNpc`
  (params (other :type "Actor Object Reference"))
  (if (`self.ActorHasTag` other "Player")
    (set `self.isPoisoned` true)))

(fn `TryToSpreadPoison`
  (params (other :type "Actor Object Reference"))
  (bind _asbp_npc (cast `/Game/Assets/Blueprints/BP_Npc` other))
  (set `/Game/Assets/Blueprints/BP_Npc.isPoisoned` (and (`self.ActorHasTag` other "Poisonable") (`self.isPoisoned`)) _asbp_npc))

(fn `UserConstructionScript`)