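; BP_Medicine is a medicine actor that calls DecreaseSize on BP_Player when the player touches it.
; Its Sphere's begin-overlap event casts to BP_Player and quits the game if DecreaseSize returns false.
; The actor stays in place after contact, as the hit event is empty and the explosion, delay and destroy chain is disconnected.
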(event `self.Sphere.OnComponentHit`
  (params (HitComponent :type "PrimitiveComponent Object Reference") (OtherActor :type "Actor Object Reference") (OtherComp :type "PrimitiveComponent Object Reference") (NormalImpulse :type "Vector Structure") (Hit :type "HitResult Structure (by ref)")))

(event `self.Sphere.OnComponentBeginOverlap`
  (params (OverlappedComponent :type "PrimitiveComponent Object Reference") (OtherActor :type "Actor Object Reference") (OtherComp :type "PrimitiveComponent Object Reference") (OtherBodyIndex :type Integer) (bFromSweep :type Boolean) (SweepResult :type "HitResult Structure (by ref)"))
  (bind _asbp_player (cast `/Game/Assets/Blueprints/BP_Player` OtherActor))
  (bind _successfull (`/Game/Assets/Blueprints/BP_Player.Decrease Size` _asbp_player))
  (if (not _successfull)
    (`KismetSystemLibrary.QuitGame` null "Quit")))

(fn `UserConstructionScript`)