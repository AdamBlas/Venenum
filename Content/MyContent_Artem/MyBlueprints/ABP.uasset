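; Enemy actor that loses HP on contact with the player (MyCharakter) and destroys itself on Tick once HP reaches zero.
; Capsule overlap starts a poison-like Delay loop that keeps draining HP, with no stop on exit.
; Mesh overlap runs a delayed, heavier damage loop, gated by a DoOnce and a flag cleared on exit.
; Both loops update the HP_Test health widget, whose component visibility follows player overlap with the Sphere.
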(event `self.ReceiveBeginPlay`
  ;[1 1 1] Get REF to UI Widget
  (bind _asmy_charakter (cast `/Game/MyContent_Artem/MyBlueprints/MyCharakter` (`GameplayStatics.GetPlayerCharacter` 0)))
  (set `self.CHArRef` _asmy_charakter)
  (bind _ashp_test (cast `/Game/MyContent_Artem/MyBlueprints/HP_Test` (`WidgetComponent.GetUserWidgetObject` (`self.HP_widget`))))
  (set `self.HealthWidgetRef` _ashp_test))

(event `self.ReceiveTick`
  (params (DeltaSeconds :type "Float (single-precision)"))
  (if (<= (`self.hp`) 0.0)
    (`self.K2_DestroyActor`)))

(event `self.CapsuleComponent.OnComponentBeginOverlap`
  (params (OverlappedComponent :type "PrimitiveComponent Object Reference") (OtherActor :type "Actor Object Reference") (OtherComp :type "PrimitiveComponent Object Reference") (OtherBodyIndex :type Integer) (bFromSweep :type Boolean) (SweepResult :type "HitResult Structure (by ref)"))
  (bind _healthwidgetref (`self.HealthWidgetRef`))
  ;[1 1 1] Poison Enemy by Gamecharakter
  (cast `/Game/MyContent_Artem/MyBlueprints/MyCharakter` OtherActor)
  (set `/Game/MyContent_Artem/MyBlueprints/HP_Test.Visability` "Visible" _healthwidgetref)
  (bind _output_get (set `self.hp` (- (`self.hp`) 1.0) :!label _label))
  (set `/Game/MyContent_Artem/MyBlueprints/HP_Test.Health` _output_get _healthwidgetref)
  (`KismetSystemLibrary.Delay` 0.2)
  (goto _label))

(event `self.Mesh.OnComponentBeginOverlap`
  (params (OverlappedComponent :type "PrimitiveComponent Object Reference") (OtherActor :type "Actor Object Reference") (OtherComp :type "PrimitiveComponent Object Reference") (OtherBodyIndex :type Integer) (bFromSweep :type Boolean) (SweepResult :type "HitResult Structure (by ref)"))
  ;[1 1 1] Logic of our gamecharakter interact with enemy
  (cast `/Game/MyContent_Artem/MyBlueprints/MyCharakter` OtherActor)
  (set `self.Condition` true)
  (`/Engine/EditorBlueprintResources/StandardMacros.DoOnce` false :!label _label_2
    (:`Completed`
      (`KismetSystemLibrary.Delay` 1.0)
      (if (`self.Condition`) :!label _label_3
        (bind _output_get (set `self.hp` (- (`self.hp`) 5.0)))
        (set `/Game/MyContent_Artem/MyBlueprints/HP_Test.Health` _output_get (`self.HealthWidgetRef`))
        (`KismetSystemLibrary.Delay` 0.5)
        (goto _label_3)))))

(event `self.Mesh.OnComponentEndOverlap`
  (params (OverlappedComponent :type "PrimitiveComponent Object Reference") (OtherActor :type "Actor Object Reference") (OtherComp :type "PrimitiveComponent Object Reference") (OtherBodyIndex :type Integer))
  ;[1 1 1] Logic of our gamecharakter interact with enemy
  (cast `/Game/MyContent_Artem/MyBlueprints/MyCharakter` OtherActor)
  (set `self.Condition` false)
  (goto _label_2 :!via `Reset`))

(event `self.Sphere.OnComponentBeginOverlap`
  (params (OverlappedComponent :type "PrimitiveComponent Object Reference") (OtherActor :type "Actor Object Reference") (OtherComp :type "PrimitiveComponent Object Reference") (OtherBodyIndex :type Integer) (bFromSweep :type Boolean) (SweepResult :type "HitResult Structure (by ref)"))
  ;[1 1 1] Wisibility of HP Widget
  (cast `/Game/MyContent_Artem/MyBlueprints/MyCharakter` OtherActor)
  (`SceneComponent.SetVisibility` (`self.HP_widget`) true false))

(event `self.Sphere.OnComponentEndOverlap`
  (params (OverlappedComponent :type "PrimitiveComponent Object Reference") (OtherActor :type "Actor Object Reference") (OtherComp :type "PrimitiveComponent Object Reference") (OtherBodyIndex :type Integer))
  ;[1 1 1] Wisibility of HP Widget
  (cast `/Game/MyContent_Artem/MyBlueprints/MyCharakter` OtherActor)
  (`SceneComponent.SetVisibility` (`self.HP_widget`) false false))

(fn `UserConstructionScript`)